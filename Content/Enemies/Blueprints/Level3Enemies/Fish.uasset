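; Level 3 fish enemy that knocks one pizza ingredient out of the player when they touch it.
; On collision overlap it checks the player's counts in fixed priority (dough, tomato, cheese, garlic, mushroom, sausage) and decrements the first non-zero one.
; It spawns that ingredient at its Arrow component, then adds a random yaw to its root.
; Nothing happens when the player carries none of these.
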(event OnComponentBeginOverlap(Collision)
  (params (OverlappedComponent :type Primitive%20Component%20Object%20Reference) (OtherActor :type Actor%20Object%20Reference) (OtherComp :type Primitive%20Component%20Object%20Reference) (OtherBodyIndex :type Integer) (bFromSweep :type Boolean) (SweepResult :type Hit%20Result%20Structure%20%28by%20ref%29))
  (bind _arrow (Variables|Default|GetArrow))
  (bind _returnvalue (Transformation|GetWorldTransform _arrow))
  (bind _asbp_third_person_character_3 (Utilities|Casting|CastToBP_ThirdPersonCharacter3 OtherActor))
  (bind _output_get (Variables|Default|SetPlayer _asbp_third_person_character_3))
  (if (> (Variables|/Game/ThirdPerson/Blueprints/BP_ThirdPersonCharacter3.BP_ThirdPersonCharacter3_C|GetDoughCount _output_get) 0)
    (Variables|/Game/ThirdPerson/Blueprints/BP_ThirdPersonCharacter3.BP_ThirdPersonCharacter3_C|SetDoughCount _output_get (- (Variables|/Game/ThirdPerson/Blueprints/BP_ThirdPersonCharacter3.BP_ThirdPersonCharacter3_C|GetDoughCount _output_get) 1))
    (Game|SpawnActorfromClass "/Game/FoodItems/Level3Ingredients/Dough.Dough_C" _returnvalue "Undefined" "MultiplyWithRoot" 0 0)
    (Transformation|AddLocalRotation (Variables|Default|GetDefaultSceneRoot) (Math|Rotator|MakeRotator 0.0 0.0 (Math|Random|RandomFloatinRange 0.0 3.6e+02)) false false :!label _label)
    (elif (> (Variables|/Game/ThirdPerson/Blueprints/BP_ThirdPersonCharacter3.BP_ThirdPersonCharacter3_C|GetTomatoCount _asbp_third_person_character_3) 0)
      (Variables|/Game/ThirdPerson/Blueprints/BP_ThirdPersonCharacter3.BP_ThirdPersonCharacter3_C|SetTomatoCount _output_get (- (Variables|/Game/ThirdPerson/Blueprints/BP_ThirdPersonCharacter3.BP_ThirdPersonCharacter3_C|GetTomatoCount _asbp_third_person_character_3) 1))
      (Game|SpawnActorfromClass "/Game/FoodItems/Level3Ingredients/TomatoIngredient3.TomatoIngredient3_C" _returnvalue "Undefined" "MultiplyWithRoot" 0 0)
      (goto _label)
      (elif (> (Variables|/Game/ThirdPerson/Blueprints/BP_ThirdPersonCharacter3.BP_ThirdPersonCharacter3_C|GetCheeseCount _asbp_third_person_character_3) 0)
        (Variables|/Game/ThirdPerson/Blueprints/BP_ThirdPersonCharacter3.BP_ThirdPersonCharacter3_C|SetCheeseCount _output_get (- (Variables|/Game/ThirdPerson/Blueprints/BP_ThirdPersonCharacter3.BP_ThirdPersonCharacter3_C|GetCheeseCount _asbp_third_person_character_3) 1))
        (Game|SpawnActorfromClass "/Game/FoodItems/Level3Ingredients/Cheese3.Cheese3_C" _returnvalue "Undefined" "MultiplyWithRoot" 0 0)
        (goto _label)
        (elif (> (Variables|/Game/ThirdPerson/Blueprints/BP_ThirdPersonCharacter3.BP_ThirdPersonCharacter3_C|GetGarlicCount (Variables|Default|GetPlayer)) 0)
          (Variables|/Game/ThirdPerson/Blueprints/BP_ThirdPersonCharacter3.BP_ThirdPersonCharacter3_C|SetGarlicCount (Variables|Default|GetPlayer) (- (Variables|/Game/ThirdPerson/Blueprints/BP_ThirdPersonCharacter3.BP_ThirdPersonCharacter3_C|GetGarlicCount (Variables|Default|GetPlayer)) 1))
          (Game|SpawnActorfromClass "/Game/FoodItems/Level3Ingredients/Garlic.Garlic_C" _returnvalue "Undefined" "MultiplyWithRoot" 0 0)
          (goto _label)
          (elif (> (Variables|/Game/ThirdPerson/Blueprints/BP_ThirdPersonCharacter3.BP_ThirdPersonCharacter3_C|GetMushroomCount (Variables|Default|GetPlayer)) 0)
            (Variables|/Game/ThirdPerson/Blueprints/BP_ThirdPersonCharacter3.BP_ThirdPersonCharacter3_C|SetMushroomCount (Variables|Default|GetPlayer) (- (Variables|/Game/ThirdPerson/Blueprints/BP_ThirdPersonCharacter3.BP_ThirdPersonCharacter3_C|GetMushroomCount (Variables|Default|GetPlayer)) 1))
            (Game|SpawnActorfromClass "/Game/FoodItems/Level3Ingredients/Mushroom.Mushroom_C" _returnvalue "Undefined" "MultiplyWithRoot" 0 0)
            (goto _label)
            (elif (> (Variables|/Game/ThirdPerson/Blueprints/BP_ThirdPersonCharacter3.BP_ThirdPersonCharacter3_C|GetSausageCount (Variables|Default|GetPlayer)) 0)
              (Variables|/Game/ThirdPerson/Blueprints/BP_ThirdPersonCharacter3.BP_ThirdPersonCharacter3_C|SetSausageCount (Variables|Default|GetPlayer) (- (Variables|/Game/ThirdPerson/Blueprints/BP_ThirdPersonCharacter3.BP_ThirdPersonCharacter3_C|GetSausageCount (Variables|Default|GetPlayer)) 1))
              (Game|SpawnActorfromClass "/Game/FoodItems/Level3Ingredients/Sausage.Sausage_C" _returnvalue "Undefined" "MultiplyWithRoot" 0 0)
              (goto _label))))))))

(event EventBeginPlay)

(event Collision|EventActorBeginOverlap
  (params (OtherActor :type Actor%20Object%20Reference)))

(event EventTick
  (params (DeltaSeconds :type Float%20%28single-precision%29)))

(fn ConstructionScript)