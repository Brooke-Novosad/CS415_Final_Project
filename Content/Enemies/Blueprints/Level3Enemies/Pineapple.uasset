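; Pineapple is a Level 3 enemy that shuttles back and forth along the X axis while spinning.
; On BeginPlay, a delayed custom loop runs a limited number of passes, each calling MoveForward and MoveBack with pauses between.
; Each move uses a timeline to lerp a swept location offset from the current position, toward negative X then back.
; Tick applies local pitch rotation, whose direction flips as each move finishes.
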(event Custom|move%20forward
  (bind _returnvalue (Transformation|GetActorLocation))
  (bind _output_get (Variables|Default|SetStart (+ _returnvalue "")))
  (bind _output_get_2 (Variables|Default|SetEnd (+ _returnvalue "-400.000000,0.000000,0.000000")))
  (bind _newtrack_0 (Timeline|Timeline PlayFromStart)
    (:Update
      (Transformation|SetActorLocation (Math|Vector|Lerp(Vector) _output_get _output_get_2 _newtrack_0) true false))
    (:Finished
      (Variables|Default|Setrotation -5.0))))

(event Custom|move%20back
  (bind _returnvalue (Transformation|GetActorLocation))
  (bind _output_get (Variables|Default|SetStart (+ _returnvalue "")))
  (bind _output_get_2 (Variables|Default|SetEnd (+ _returnvalue "400.000000,0.000000,0.000000")))
  (bind _newtrack_0 (Timeline|Timeline_0 PlayFromStart)
    (:Update
      (Transformation|SetActorLocation (Math|Vector|Lerp(Vector) _output_get _output_get_2 _newtrack_0) true false))
    (:Finished
      (Variables|Default|Setrotation 5.0))))

(event EventBeginPlay
  (Utilities|CustomLoopwithDelay 0 3 10.1
    (:Loop%20Body
      (CallFunction|MoveForward)
      (Utilities|FlowControl|Delay 5.0)
      (CallFunction|MoveBack)
      (Utilities|FlowControl|Delay 5.0))))

(event Collision|EventActorBeginOverlap
  (params (OtherActor :type Actor%20Object%20Reference)))

(event EventTick
  (params (DeltaSeconds :type Float%20%28single-precision%29))
  (Transformation|AddActorLocalRotation (Math|Rotator|MakeRotator 0.0 (Variables|Default|Getrotation) 0.0) false false))

(fn ConstructionScript)