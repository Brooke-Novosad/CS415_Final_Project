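; Broccoli is a Level 1 enemy that knocks a collected ingredient out of the player on contact.
; When its collision component overlaps BP_ThirdPersonCharacter, it decrements the first non-zero count, checked in the order flour, egg, then sugar.
; It then spawns the matching ingredient actor at its Arrow component's transform.
; If the player holds none of these, it only prints a debug string.
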(event OnComponentBeginOverlap(CollisionBroccoli)
  (params (OverlappedComponent :type Primitive%20Component%20Object%20Reference) (OtherActor :type Actor%20Object%20Reference) (OtherComp :type Primitive%20Component%20Object%20Reference) (OtherBodyIndex :type Integer) (bFromSweep :type Boolean) (SweepResult :type Hit%20Result%20Structure%20%28by%20ref%29))
  (bind _arrow (Variables|Default|GetArrow))
  (bind _returnvalue (Transformation|GetWorldTransform _arrow))
  (bind _asbp_third_person_character (Utilities|Casting|CastToBP_ThirdPersonCharacter OtherActor))
  (if (> (Variables|/Game/ThirdPerson/Blueprints/BP_ThirdPersonCharacter.BP_ThirdPersonCharacter_C|GetFlourCount _asbp_third_person_character) 0)
    (Variables|/Game/ThirdPerson/Blueprints/BP_ThirdPersonCharacter.BP_ThirdPersonCharacter_C|SetFlourCount _asbp_third_person_character (- (Variables|/Game/ThirdPerson/Blueprints/BP_ThirdPersonCharacter.BP_ThirdPersonCharacter_C|GetFlourCount _asbp_third_person_character) 1))
    (Game|SpawnActorfromClass "/Game/FoodItems/Level1Ingredients/FlourIngredient.FlourIngredient_C" _returnvalue "Undefined" "MultiplyWithRoot" 0 0)
    (elif (> (Variables|/Game/ThirdPerson/Blueprints/BP_ThirdPersonCharacter.BP_ThirdPersonCharacter_C|GetEggCount _asbp_third_person_character) 0)
      (Variables|/Game/ThirdPerson/Blueprints/BP_ThirdPersonCharacter.BP_ThirdPersonCharacter_C|SetEggCount _asbp_third_person_character (- (Variables|/Game/ThirdPerson/Blueprints/BP_ThirdPersonCharacter.BP_ThirdPersonCharacter_C|GetEggCount _asbp_third_person_character) 1))
      (Game|SpawnActorfromClass "/Game/FoodItems/Level1Ingredients/EggIngredient.EggIngredient_C" _returnvalue "Undefined" "MultiplyWithRoot" 0 0)
      (elif (> (Variables|/Game/ThirdPerson/Blueprints/BP_ThirdPersonCharacter.BP_ThirdPersonCharacter_C|GetSugarCount _asbp_third_person_character) 0)
        (Variables|/Game/ThirdPerson/Blueprints/BP_ThirdPersonCharacter.BP_ThirdPersonCharacter_C|SetSugarCount _asbp_third_person_character (- (Variables|/Game/ThirdPerson/Blueprints/BP_ThirdPersonCharacter.BP_ThirdPersonCharacter_C|GetSugarCount _asbp_third_person_character) 1))
        (Game|SpawnActorfromClass "/Game/FoodItems/Level1Ingredients/Sugar.Sugar_C" _returnvalue "Undefined" "MultiplyWithRoot" 0 0)
        (else
          (Development|PrintString "no"))))))

(event EventBeginPlay)

(event Collision|EventActorBeginOverlap
  (params (OtherActor :type Actor%20Object%20Reference)))

(event EventTick
  (params (DeltaSeconds :type Float%20%28single-precision%29)))

(fn ConstructionScript)