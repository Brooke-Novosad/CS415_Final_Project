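; Cucumber is a Level 1 enemy that rolls back and forth along a fixed path and hurts the player on contact.
; On BeginPlay it derives an end point from its forward arrow, then a delayed loop macro triggers a few timed out-and-back moves.
; Two timelines lerp its location with sweep, and each flips the pitch spin applied every Tick when it finishes.
; Collision overlap with BP_ThirdPersonCharacter1 calls DecreaseHealth.
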(event OnComponentBeginOverlap(Collision)
  (params (OverlappedComponent :type Primitive%20Component%20Object%20Reference) (OtherActor :type Actor%20Object%20Reference) (OtherComp :type Primitive%20Component%20Object%20Reference) (OtherBodyIndex :type Integer) (bFromSweep :type Boolean) (SweepResult :type Hit%20Result%20Structure%20%28by%20ref%29))
  (bind _asbp_third_person_character_1 (Utilities|Casting|CastToBP_ThirdPersonCharacter1 OtherActor))
  (Default|DecreaseHealth _asbp_third_person_character_1))

(event Custom|move%20forward
  (bind _newtrack_0 (Timeline|Timeline_1 PlayFromStart)
    (:Update
      (Transformation|SetActorLocation (Math|Vector|Lerp(Vector) (Variables|Default|GetStart) (Variables|Default|GetEnd) _newtrack_0) true false))
    (:Finished
      (Variables|Default|Setrotation 5.0))))

(event Custom|move%20back
  (bind _newtrack_0 (Timeline|Timeline_2 ReverseFromEnd)
    (:Update
      (Transformation|SetActorLocation (Math|Vector|Lerp(Vector) (Variables|Default|GetStart) (Variables|Default|GetEnd) _newtrack_0) true false))
    (:Finished
      (Variables|Default|Setrotation -5.0))))

(event EventBeginPlay
  (Variables|Default|SetStart (Transformation|GetActorLocation))
  (Variables|Default|SetEnd (+ (Transformation|GetActorLocation) (* (Math|Vector|GetForwardVector (Variables|Default|GetArrowForwards)) "500.000000,500.000000,1.000000")))
  (Utilities|CustomLoopwithDelay 0 3 10.1
    (:Loop%20Body
      (CallFunction|MoveForward)
      (Utilities|FlowControl|Delay 5.0)
      (CallFunction|MoveBack)
      (Utilities|FlowControl|Delay 5.0))))

(event Collision|EventActorBeginOverlap
  (params (OtherActor :type Actor%20Object%20Reference)))

(event EventTick
  (params (DeltaSeconds :type Float%20%28single-precision%29))
  (Transformation|AddActorLocalRotation (Math|Rotator|MakeRotator 0.0 (Variables|Default|Getrotation) 0.0) false false))

(fn ConstructionScript)