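; Campfire prop Blueprint that acts as a trigger for a jigsaw puzzle, gated by collected ingredients.
; Box overlap checks the third-person character for at least three each of dough, cheese, water and tomato, showing a timed warning widget if short.
; Otherwise it creates the jigsaw widget, stops player movement and switches to UI-only input with a cursor.
; An existing puzzle widget is reused, skipping the ingredient check.
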(event OnComponentBeginOverlap(Box)
  (params (OverlappedComponent :type Primitive%20Component%20Object%20Reference) (OtherActor :type Actor%20Object%20Reference) (OtherComp :type Primitive%20Component%20Object%20Reference) (OtherBodyIndex :type Integer) (bFromSweep :type Boolean) (SweepResult :type Hit%20Result%20Structure%20%28by%20ref%29))
  (bind _returnvalue (Game|GetPlayerController 0))
  (Utilities|IsValid (Variables|Default|GetPuzzleWidget)
    (:Is%20Valid
      (UserInterface|Viewport|AddtoViewport (Variables|Default|GetPuzzleWidget) 0 :!label _label)
      (Components|Movement|StopMovementImmediately (Variables|/Script/Engine.Character|GetCharacterMovement (Game|GetPlayerCharacter 0)))
      (Input|SetInputModeUIOnly _returnvalue (Variables|Default|GetPuzzleWidget) "DoNotLock" false)
      (Variables|/Script/Engine.PlayerController|SetbShowMouseCursor _returnvalue true)
      (Development|PrintString "Reached Camp Fire, Puzzle1 Time"))
    (:Is%20Not%20Valid
      (bind _asbp_third_person_character_2 (Utilities|Casting|CastToBP_ThirdPersonCharacter2 (Game|GetPlayerCharacter 0)))
      (if (Math|Boolean|ANDBoolean (>= (Variables|/Game/ThirdPerson/Blueprints/BP_ThirdPersonCharacter2.BP_ThirdPersonCharacter2_C|GetDoughCount _asbp_third_person_character_2) 3) (>= (Variables|/Game/ThirdPerson/Blueprints/BP_ThirdPersonCharacter2.BP_ThirdPersonCharacter2_C|GetCheeseCount _asbp_third_person_character_2) 3) (>= (Variables|/Game/ThirdPerson/Blueprints/BP_ThirdPersonCharacter2.BP_ThirdPersonCharacter2_C|GetWaterCount _asbp_third_person_character_2) 3) (>= (Variables|/Game/ThirdPerson/Blueprints/BP_ThirdPersonCharacter2.BP_ThirdPersonCharacter2_C|GetTomatoCount _asbp_third_person_character_2) 3))
        (bind _returnvalue_2 (UserInterface|CreateWidget "/Game/JigsawWidget.JigsawWidget_C"))
        (Variables|Default|SetPuzzleWidget _returnvalue_2)
        (goto _label)
        (else
          (bind _returnvalue_3 (UserInterface|CreateWidget "/Game/ThirdPerson/Blueprints/Notenoughitems.Notenoughitems_C"))
          (UserInterface|Viewport|AddtoViewport _returnvalue_3 0)
          (Utilities|FlowControl|Delay 3.0)
          (Widget|RemovefromParent _returnvalue_3))))))

(event EventBeginPlay)

(event Collision|EventActorBeginOverlap
  (params (OtherActor :type Actor%20Object%20Reference)))

(event EventTick
  (params (DeltaSeconds :type Float%20%28single-precision%29)))

(fn ConstructionScript)